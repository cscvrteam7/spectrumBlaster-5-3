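; Turret actor that tracks and shoots at a ThirdPersonCharacter2 while it is inside the Collision volume.
; Overlap begin and end open and close a Tick gate, which turns the Head toward the character's mesh using RInterpTo with a fixed delta time, making turning frame-rate dependent.
; SpawnProjectile, called every gated tick, uses a game-time cooldown to spawn a FirstPersonProjectile at the Arrow and play a sound.
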(event `self.ReceiveTick`
  (params (DeltaSeconds :type "Float (single-precision)"))
  (bind _head (`self.head`))
  (`/Engine/EditorBlueprintResources/StandardMacros.Gate` true :!label _label
    (:`Exit`
      (`SceneComponent.K2_SetWorldRotation` (`self.head`) (`KismetMathLibrary.RInterpTo` (`SceneComponent.K2_GetComponentRotation` _head) (`KismetMathLibrary.FindLookAtRotation` (`SceneComponent.K2_GetComponentLocation` _head) (`SceneComponent.K2_GetComponentLocation` (`Character.Mesh` (stale `self.collision.OnComponentBeginOverlap` _asthird_person_character_2)))) 1.0 (`self.turret rot speed`)) false false)
      (`self.spawnProjectile`))))

(event `self.collision.OnComponentBeginOverlap`
  (params (OverlappedComponent :type "PrimitiveComponent Object Reference") (OtherActor :type "Actor Object Reference") (OtherComp :type "PrimitiveComponent Object Reference") (OtherBodyIndex :type Integer) (bFromSweep :type Boolean) (SweepResult :type "HitResult Structure (by ref)"))
  (bind _asthird_person_character_2 (cast `/Game/Mannequin/ThirdPersonCharacter2` OtherActor))
  (goto _label :!via `Open`))

(event `self.collision.OnComponentEndOverlap`
  (params (OverlappedComponent :type "PrimitiveComponent Object Reference") (OtherActor :type "Actor Object Reference") (OtherComp :type "PrimitiveComponent Object Reference") (OtherBodyIndex :type Integer))
  (cast `/Game/Mannequin/ThirdPersonCharacter2` OtherActor)
  (goto _label :!via `Close`))

(fn `spawnProjectile`
  (bind _returnvalue (`KismetSystemLibrary.GetGameTimeInSeconds`))
  (if (> _returnvalue (`self.gameFire`))
    (set `self.gameFire` (+ _returnvalue (`self.fireDelay`)))
    (`|SpawnActorFromClass` "/Game/Mannequin/FirstPersonProjectile.FirstPersonProjectile_C" (`SceneComponent.K2_GetComponentToWorld` (`self.Arrow`)) "Undefined" "OverrideRootScale")
    (`GameplayStatics.PlaySoundAtLocation` "/Game/Bass-Drum-1.Bass-Drum-1" (`self.K2_GetActorLocation`))))

(fn `UserConstructionScript`)